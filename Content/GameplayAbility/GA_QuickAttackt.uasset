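; Quick attack gameplay ability that applies GE_VirusEffect to pawns inside the avatar's damage collision.
; On activation it loops over pawns overlapping the avatar's DamageCollisionEvaluator component and prints each name.
; The owner's ability system applies the effect to each pawn, but the spec and context come from the target's own AbilitySystemComponent.
; The graph never commits or ends the ability.
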(event `self.K2_ActivateAbility`
  (for _array_element (`PrimitiveComponent.GetOverlappingActors` (`Actor.GetComponentByClass` (`self.GetAvatarActorFromActorInfo`) "/Script/UTHUB_GAS2025.DamageCollisionEvaluator") "/Script/Engine.Pawn")
    (`KismetSystemLibrary.PrintString` (`KismetSystemLibrary.GetDisplayName` _array_element))
    (bind _returnvalue (`Actor.GetComponentByClass` _array_element "/Script/GameplayAbilities.AbilitySystemComponent"))
    (`AbilitySystemComponent.BP_ApplyGameplayEffectSpecToTarget` (`self.GetAbilitySystemComponentFromActorInfo`) (`AbilitySystemComponent.MakeOutgoingSpec` _returnvalue "/Game/GameplayEffects/Ejercicio3/GE_VirusEffect.GE_VirusEffect_C" 0.0 (`AbilitySystemComponent.MakeEffectContext` _returnvalue)) _returnvalue)))