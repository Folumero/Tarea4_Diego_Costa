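; GA_Trace is a gameplay ability that runs a timed look phase (HabilitarMirada) and a recovery period.
; After a brief delay, a successful HabilitarMirada starts a timer for the ability duration, which then calls ResRotacionCameraBoom.
; A recovery timer follows and ends the ability.
; Otherwise, it removes the Character.CantTrace tag from the avatar character without calling EndAbility.
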(event `self.K2_ActivateAbility`
  (`KismetSystemLibrary.Delay` 0.01)
  (if (`self.bHabilitarMirada`)
    (`KismetSystemLibrary.K2_SetTimerDelegate` (delegate `CustomEvent`) (`self.TiempoHabilidad`))
    (else
      (bind _ascharacter (cast `Character` (`self.GetAvatarActorFromActorInfo`)))
      (`AbilitySystemBlueprintLibrary.RemoveLooseGameplayTags` _ascharacter (`BlueprintGameplayTagLibrary.MakeGameplayTagContainerFromArray` (`|MakeArray` (struct :`TagName` "Character.CantTrace") :!type "GameplayTag Structure"))))))

(event `CustomEvent`
  (`self.ResRotacionCameraBoom`)
  (`KismetSystemLibrary.K2_SetTimerDelegate` (delegate `CustomEvent_0`) (`self.TiempoRecuperacion`)))

(event `CustomEvent_0`
  (`self.K2_EndAbility`))