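; Gameplay ability that makes the avatar Character jump and blocks attacking and blocking until it ends.
; On activation it jumps, removes the loose CanAttackt and CanBlock tags, and binds to the character's actor-hit event.
; A hit restores both tags and ends the ability, except a hit on a "suelo"-tagged actor while dashing, which delays this by a timer meant to match the dash duration.
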(event `self.K2_ActivateAbility`
  (bind _ascharacter (cast `Character` (`self.GetAvatarActorFromActorInfo`)))
  (`Character.Jump` _ascharacter)
  (`AbilitySystemBlueprintLibrary.RemoveLooseGameplayTags` _ascharacter (`BlueprintGameplayTagLibrary.MakeGameplayTagContainerFromArray` (`|MakeArray` (struct :`TagName` "Character.CanAttackt") (struct :`TagName` "Character.CanBlock") :!type "GameplayTag Structure")))
  (add `Actor.OnActorHit` _ascharacter (delegate `CustomEvent`)))

(event `CustomEvent_0`
  (`AbilitySystemBlueprintLibrary.RemoveLooseGameplayTags` (stale `self.K2_ActivateAbility` _ascharacter) (`BlueprintGameplayTagLibrary.MakeGameplayTagContainerFromArray` (`|MakeArray` (struct :`TagName` "Character.CanAttackt") (struct :`TagName` "Character.CanBlock") :!type "GameplayTag Structure")))
  (`AbilitySystemBlueprintLibrary.AddLooseGameplayTags` (stale `self.K2_ActivateAbility` _ascharacter) (`BlueprintGameplayTagLibrary.MakeGameplayTagContainerFromArray` (`|MakeArray` (struct :`TagName` "Character.CanAttackt") (struct :`TagName` "Character.CanBlock") :!type "GameplayTag Structure")))
  (`self.K2_EndAbility`))

(event `CustomEvent`
  (params (SelfActor :type "Actor Object Reference") (OtherActor :type "Actor Object Reference") (NormalImpulse :type "Vector Structure") (Hit :type "HitResult Structure (by ref)"))
  (bind _ascharacter (cast `Character` (`self.GetAvatarActorFromActorInfo`)))
  (if (and (`Actor.ActorHasTag` Hit_HitActor "suelo") (`GameplayTagAssetInterface.HasAnyMatchingGameplayTags` (`Actor.GetComponentByClass` _ascharacter "/Script/GameplayAbilities.AbilitySystemComponent") (`BlueprintGameplayTagLibrary.MakeGameplayTagContainerFromTag` (struct :`TagName` "Character.IsDashing"))))
    ;[1 1 1] MismoTiempoQueElDash
    (`KismetSystemLibrary.K2_SetTimerDelegate` (delegate `CustomEvent_0`) 1.0)
    (else
      (`AbilitySystemBlueprintLibrary.AddLooseGameplayTags` (stale `self.K2_ActivateAbility` _ascharacter) (`BlueprintGameplayTagLibrary.MakeGameplayTagContainerFromArray` (`|MakeArray` (struct :`TagName` "Character.CanAttackt") (struct :`TagName` "Character.CanBlock") :!type "GameplayTag Structure")))
      (`self.K2_EndAbility`))))